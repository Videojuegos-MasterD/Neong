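; Player controller for a two-paddle, Pong-style game, moving both Player actors vertically within a clamped height.
; On BeginPlay it identifies the paddles by display name and enables movement after a short delay.
; Input axes drive each paddle at its own speed, while an AI flag replaces Player 2 input with a Tick-driven MoveComponentTo that trails the Ball's height.
; Escape quits the game.
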(event `self.ReceiveBeginPlay`
  ;[0.3594 0.3594 0.3594] Set up players and controllers
  (bind _outactors (`GameplayStatics.GetAllActorsOfClass` "/Game/Blueprints/Player.Player_C"))
  (for _array_element _outactors
    (if (`KismetStringLibrary.EqualEqual_StrStr` (`KismetSystemLibrary.GetDisplayName` _array_element) "Player1")
      (set `self.Player1` _array_element)
      (else
        (set `self.Player2` _array_element)))
    (`KismetSystemLibrary.Delay` 1.0)
    (set `self.CanMove` true)))

(event `InputAxis|Player1Move`
  (params (AxisValue :type "Float (single-precision)"))
  (bind _maxheigh (`self.MaxHeigh`))
  (bind _player1 (`self.Player1`))
  (bind (_returnvalue_x _returnvalue_y _returnvalue_z) (`KismetMathLibrary.BreakVector` (+ (`self.K2_GetActorLocation` _player1) (`KismetMathLibrary.MakeVector` 0.0 0.0 (* AxisValue (`self.SpeedP1`))))))
  ;[0.125 1 0.125] Player 1 movement
  (if (`self.CanMove`)
    (`self.K2_SetActorLocation` _player1 (`KismetMathLibrary.MakeVector` _returnvalue_x _returnvalue_y (`KismetMathLibrary.FClamp` _returnvalue_z (* _maxheigh -1.0) _maxheigh)) false false)))

(event `Key|Escape`
  (params (Key :type "Key Structure"))
  ;[0 1 1] Pause
  (:`Pressed`
    (`KismetSystemLibrary.QuitGame` null "Quit")))

(event `InputAxis|Player2Move`
  (params (AxisValue :type "Float (single-precision)"))
  (bind _maxheigh (`self.MaxHeigh`))
  (bind _player2 (`self.Player2`))
  (bind (_returnvalue_x _returnvalue_y _returnvalue_z) (`KismetMathLibrary.BreakVector` (+ (`self.K2_GetActorLocation` _player2) (`KismetMathLibrary.MakeVector` 0.0 0.0 (* AxisValue (`self.SpeedP2`))))))
  ;[0.1216 1 0.1216] Player 2 movement
  (if (`self.CanMove`)
    (if (not (`self.AI`))
      (`self.K2_SetActorLocation` _player2 (`KismetMathLibrary.MakeVector` _returnvalue_x _returnvalue_y (`KismetMathLibrary.FClamp` _returnvalue_z (* _maxheigh -1.0) _maxheigh)) false false))))

(event `self.ReceiveTick`
  (params (DeltaSeconds :type "Float (single-precision)"))
  (bind _player2 (`self.Player2`))
  (bind _maxheigh (`self.MaxHeigh`))
  (bind (_returnvalue_x _returnvalue_y) (`KismetMathLibrary.BreakVector` (`self.K2_GetActorLocation` _player2)))
  ;[0.1216 1 0.1216] AI movement
  (if (`self.AI`)
    (if (`self.CanMove`)
      (bind _returnvalue (`GameplayStatics.GetActorOfClass` "/Game/Blueprints/Ball.Ball_C"))
      (bind (_returnvalue_x_2 _returnvalue_y_2 _returnvalue_z) (`KismetMathLibrary.BreakVector` (`self.K2_GetActorLocation` _returnvalue)))
      (`KismetSystemLibrary.MoveComponentTo` (`/Game/Blueprints/Player.Player` (cast `/Game/Blueprints/Player` _player2 :!pure true)) (`KismetMathLibrary.MakeVector` _returnvalue_x _returnvalue_y (`KismetMathLibrary.FClamp` _returnvalue_z (* _maxheigh -1.0) _maxheigh)) (struct) false false (`self.DelayAI`)))))

(fn `UserConstructionScript`)