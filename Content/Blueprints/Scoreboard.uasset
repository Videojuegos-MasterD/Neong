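; Scoreboard actor that counts one side's goals up to a winning score and animates the lead against a linked EnemyScoreboard.
; Each Goal increments the score, then chained timelines slide the number before its digit mesh is swapped and a particle effect fires.
; Taking the lead, match point or victory starts a self-restarting timeline that pulses the root scale while Winning.
; Scoring also updates the enemy board's Winning flag, controlling its pulse.
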(event `self.ReceiveBeginPlay`
  ;[0.3021 0.3021 0.3021] Set scoreboards to 0
  (set `self.SpeakerInitialScale` (`SceneComponent.K2_GetComponentScale` (`self.DefaultSceneRoot`)))
  (`self.ResetScoreboard`))

(event `ResetScoreboard`
  ;[0.1216 0.3059 1] Reset the scoreboard at 0
  (`StaticMeshComponent.SetStaticMesh` (`self.ScoreNumber`) "/Game/ThirdParty/Numbers/0.0"))

(event `Goal`
  (bind (_scorenumberinitiallocation_x _scorenumberinitiallocation_y _scorenumberinitiallocation_z) (`KismetMathLibrary.BreakVector` (`self.ScoreNumberInitialLocation`)))
  (bind (_scorenumberinitiallocation_x_2 _scorenumberinitiallocation_y_2 _scorenumberinitiallocation_z_2) (`KismetMathLibrary.BreakVector` (`self.ScoreNumberInitialLocation`)))
  (bind _particlesystem (`self.ParticleSystem`))
  (bind _enemyscoreboard (`self.EnemyScoreboard`))
  (bind _enemyscoreboard_2 (`self.EnemyScoreboard`))
  ;[0.06456 0.1178 0.6198] Changes the scoreboards at goal
  (`|ExecutionSequence`
    (:`then_0`
      (set `self.Score` (+ (`self.Score`) 1))
      (set `self.ScoreNumberInitialLocation` (`SceneComponent.RelativeLocation` (`self.ScoreNumber`)))
      (`KismetSystemLibrary.Delay` 0.5)
      (bind (_direction _alpha) (`Timeline|ScoreNumberAnim` :!via `PlayFromStart`)
        (:`Update`
          (`SceneComponent.K2_SetRelativeLocation` (`self.ScoreNumber`) (`KismetMathLibrary.VLerp` (`self.ScoreNumberInitialLocation`) (`KismetMathLibrary.MakeVector` _scorenumberinitiallocation_x_2 (+ _scorenumberinitiallocation_y_2 -50.0) _scorenumberinitiallocation_z_2) _alpha) false false))
        (:`Finished`
          (bind (_direction_2 _alpha_2) (`Timeline|ScoreNumberAnim2` :!via `PlayFromStart`)
            (:`Update`
              (`SceneComponent.K2_SetRelativeLocation` (`self.ScoreNumber`) (`KismetMathLibrary.VLerp` (`self.ScoreNumberInitialLocation`) (`KismetMathLibrary.MakeVector` _scorenumberinitiallocation_x (+ _scorenumberinitiallocation_y -50.0) _scorenumberinitiallocation_z) _alpha_2) false false))
            (:`Finished`
              (`StaticMeshComponent.SetStaticMesh` (`self.ScoreNumber`) (select `int` (`self.Score`) :`0` (`self.0`) :`1` (`self.1`) :`2` (`self.2`) :`3` (`self.3`) :`4` (`self.4`) :`5` (`self.5`) :`6` (`self.6`) :`7` (`self.7`) :`8` (`self.8`) :`9` (`self.9`)))
              (`ActorComponent.Activate` _particlesystem false)
              (`ActorComponent.Deactivate` _particlesystem))))))
    (:`then_1`
      ;;[1 0.1137 0.07451] Animation conditions
      (if (== (`self.Score`) (- (`self.ScoreToWin`) 1))
        (set `self.1PointToWin` true)
        (`self.Advantage`)
        (set `/Game/Blueprints/Scoreboard.Winning?` (`/Game/Blueprints/Scoreboard.1PointToWin` _enemyscoreboard_2) _enemyscoreboard_2)
        (elif (== (`self.Score`) (`self.ScoreToWin`))
          (set `self.Win?` true)
          (set `/Game/Blueprints/Scoreboard.Winning?` false (`self.EnemyScoreboard`))
          (set `self.Winning?` false)
          (`self.Advantage`)
          (elif (> (`self.Score`) (`/Game/Blueprints/Scoreboard.Score` (`self.EnemyScoreboard`)))
            (`/Engine/EditorBlueprintResources/StandardMacros.DoOnce` false :!label _label
              (:`Completed`
                (`self.Advantage`)
                (set `/Game/Blueprints/Scoreboard.Winning?` false (`self.EnemyScoreboard`))))
            (else
              (`|ExecutionSequence`
                (:`then_0`
                  (goto _label :!via `Reset`))
                (:`then_1`
                  (if (== (`self.Score`) (`/Game/Blueprints/Scoreboard.Score` (`self.EnemyScoreboard`)))
                    (set `/Game/Blueprints/Scoreboard.Winning?` (`/Game/Blueprints/Scoreboard.1PointToWin` _enemyscoreboard) _enemyscoreboard)))))))))))

(event `Advantage`
  ;[1 0.4325 0.02144] Scoreboard animation
  (set `self.Winning?` true)
  (bind (_direction _alpha) (`Timeline|SpeakerAnim` :!via `PlayFromStart` :!label _label_2)
    (:`Update`
      (`SceneComponent.SetWorldScale3D` (`self.DefaultSceneRoot`) (* (`self.SpeakerInitialScale`) _alpha)))
    (:`Finished`
      (`KismetSystemLibrary.Delay` 0.001)
      (if (`self.Winning?`)
        (goto _label_2 :!via `PlayFromStart`)))))

(fn `UserConstructionScript`)