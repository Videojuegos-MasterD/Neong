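; Pong-style ball actor that bounces off players with a projectile movement component and reacts to goals.
; It spawns at a random height with a velocity picked from preset options.
; Player hits increase Y speed up to a clamp and set Z velocity from the impact offset to the hitbox, steering the return.
; On a goal, bouncing stops and a timeline eases velocity to zero, then the ball destroys itself unless Win is set.
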(event `self.ReceiveBeginPlay`
  (bind _maxheigh (`self.MaxHeigh`))
  ;[1 1 0] First spawn velocity of the ball
  (`self.K2_SetActorLocation` (`KismetMathLibrary.MakeVector` 0.0 0.0 (`KismetMathLibrary.RandomFloatInRange` (* _maxheigh -1.0) _maxheigh)))
  (set `MovementComponent.Velocity` (`BlueprintMapLibrary.Map_Find` (`self.PossibleVelocities`) (`KismetMathLibrary.RandomInteger` 3)) (`self.ProjectileMovement`)))

(event `Goal`
  ;[0 1 1] Goal event and animation
  (set `self.CanBounce?` false)
  (set `self.LastVelocity` (`MovementComponent.Velocity` (`self.ProjectileMovement`)))
  (bind (_direction _alpha) (`Timeline|Timeline` :!via `PlayFromStart`)
    (:`Update`
      (set `MovementComponent.Velocity` (`KismetMathLibrary.VLerp` (`self.LastVelocity`) (0.0 0.0 0.0) _alpha) (`self.ProjectileMovement`)))
    (:`Finished`
      (`KismetSystemLibrary.Delay` 0.3)
      (if (not (`self.Win?`))
        (`self.K2_DestroyActor`)))))

(event `self.ProjectileMovement.OnProjectileBounce`
  (params (ImpactResult :type "HitResult Structure (by ref)") (ImpactVelocity :type "Vector Structure (by ref)"))
  (bind (_bblockinghit _binitialoverlap _time _distance _location _impactpoint _normal _impactnormal _physmat _hitactor) (`GameplayStatics.BreakHitResult` ImpactResult))
  (bind _speedincrement (`self.SpeedIncrement`))
  (bind _maxvelocity (`self.MaxVelocity`))
  (bind _projectilemovement (`self.ProjectileMovement`))
  (bind (_velocity_x _velocity_y) (`KismetMathLibrary.BreakVector` (`MovementComponent.Velocity` _projectilemovement)))
  ;[0.1094 1 0.1094] Direction and speed of the ball when bounce
  (if (`self.CanBounce?`)
    (`GameplayStatics.PlaySound2D` "/Game/Audio/Bounce.Bounce" 1.0 1.0 0.0 null null)
    (bind _asplayer (cast `/Game/Blueprints/Player` _hitactor))
    (if (> _velocity_y 0.0)
      (set `self.Velocity` (+ _velocity_y _speedincrement))
      (else
        (set `self.Velocity` (- _velocity_y _speedincrement))))
    (bind (_returnvalue_x _returnvalue_y _returnvalue_z) (`KismetMathLibrary.BreakVector` (`SceneComponent.K2_GetComponentLocation` (`/Game/Blueprints/Player.Hitbox` _asplayer))))
    (set `MovementComponent.Velocity` (`KismetMathLibrary.MakeVector` 0.0 (`KismetMathLibrary.FClamp` (`self.Velocity`) (* _maxvelocity -1.0) _maxvelocity) (* (- (.z _impactpoint) _returnvalue_z) (`self.ImpactSensibility`))) _projectilemovement)))

(fn `UserConstructionScript`)