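; Goal trigger actor that scores when the ball's collider enters it and runs the round transition.
; A DoOnce-guarded overlap notifies the ball and the enemy scoreboard, then disables movement on the first player controller.
; After a delay, a win triggers the GUI's win event with whether the scoring team is Blue.
; Otherwise it calls NewRound on all players, spawns a new ball, restores movement and re-arms the DoOnce.
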(event `self.Col.OnComponentBeginOverlap`
  (params (OverlappedComponent :type "PrimitiveComponent Object Reference") (OtherActor :type "Actor Object Reference") (OtherComp :type "PrimitiveComponent Object Reference") (OtherBodyIndex :type Integer) (bFromSweep :type Boolean) (SweepResult :type "HitResult Structure (by ref)"))
  (bind _asscoreboard (cast `/Game/Blueprints/Scoreboard` (`self.EnemyScoreboard`) :!pure true))
  ;[1 0.09804 0.7333] Goal event
  (bind _asball (cast `/Game/Blueprints/Ball` OtherActor))
  (if (== (`/Game/Blueprints/Ball.Col` _asball) OtherComp)
    (`/Engine/EditorBlueprintResources/StandardMacros.DoOnce` false :!label _label
      (:`Completed`
        (`/Game/Blueprints/Ball.Goal` _asball)
        (`/Game/Blueprints/Scoreboard.Goal` _asscoreboard)
        (set `/Game/Blueprints/MainPlayersController.CanMove` false (cast `/Game/Blueprints/MainPlayersController` (`GameplayStatics.GetPlayerController` 0) :!pure true))
        (bind _output_get (set `/Game/Blueprints/Ball.Win?` (`/Game/Blueprints/Scoreboard.Win?` _asscoreboard) _asball))
        (if _output_get
          ;[0.0588 1 0.5655] Win event
          (`KismetSystemLibrary.Delay` 2.0)
          (bind _foundwidgets (`WidgetBlueprintLibrary.GetAllWidgetsOfClass` "/Game/Blueprints/Widgets/GUI.GUI_C"))
          (`/Game/Blueprints/Widgets/GUI.WinEvent` (`|GetArrayItem` _foundwidgets) (`KismetTextLibrary.EqualEqual_TextText` (`/Game/Blueprints/Scoreboard.Team` _asscoreboard) "Blue"))
          (else
            (`KismetSystemLibrary.Delay` 2.0)
            ;[1 0.09804 0.7333] New round event
            (bind _outactors (`GameplayStatics.GetAllActorsOfClass` "/Game/Blueprints/Player.Player_C"))
            (for _array_element _outactors
              (`/Game/Blueprints/Player.NewRound` _array_element))
            (`KismetSystemLibrary.Delay` 1.0)
            (`|SpawnActorFromClass` "/Game/Blueprints/Ball.Ball_C" (`KismetMathLibrary.MakeTransform` (0.0 0.0 0.0) (struct)) "Undefined" "OverrideRootScale" null null)
            (set `/Game/Blueprints/MainPlayersController.CanMove` true (cast `/Game/Blueprints/MainPlayersController` (`GameplayStatics.GetPlayerController` 0) :!pure true))
            (goto _label :!via `Reset`)))))))

(fn `UserConstructionScript`)