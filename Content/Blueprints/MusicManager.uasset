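; MusicManager is a Blueprint that starts and stops the game's music for the main menu and for gameplay.
; Each theme has its own event with a Play flag: true spawns a 2D sound and stores the audio component, false fades that stored component out over a short linear fade.
; The two themes are controlled independently, with no crossfade logic between them.
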(event `PlayMainMenuTheme`
  (params (`Play?` :type Boolean))
  ;[0.6115 0.1235 1] Main menu theme event
  (if `Play?`
    (bind _returnvalue (`GameplayStatics.SpawnSound2D` null 1.0 1.0 0.0 null))
    (set `self.MainMenuTheme` _returnvalue)
    (else
      (`AudioComponent.FadeOut` (`self.MainMenuTheme`) 0.5 0.0 "Linear"))))

(event `PlayGameTheme`
  (params (`Play?` :type Boolean))
  ;[0.6115 0.1235 1] Game theme event
  (if `Play?`
    (bind _returnvalue (`GameplayStatics.SpawnSound2D` null 1.0 1.0 0.0 null))
    (set `self.GameTheme` _returnvalue)
    (else
      (`AudioComponent.FadeOut` (`self.GameTheme`) 0.5 0.0 "Linear"))))

(fn `UserConstructionScript`)